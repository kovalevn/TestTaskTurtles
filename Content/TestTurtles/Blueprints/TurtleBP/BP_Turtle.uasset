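; BP_Turtle is an AI-moved turtle that travels toward a finish point in one of three patterns set by TurtleType.
; BeginPlay plays spawn effects, then starts simple, stop-and-go, or back-and-forth movement via SimpleMoveToActor, looping the latter two with delays.
; Tick pauses the attached movement sound when the turtle is nearly still.
; OnDestroy plays explosion effects, stops that sound and destroys the actor.
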(event `self.ReceiveBeginPlay`
  (bind _returnvalue (`GameplayStatics.SpawnSoundAttached` "/Game/StarterContent/Audio/Steam01_Cue.Steam01_Cue" (`self.Mesh`) "None" (0.0 0.0 0.0) (struct) "KeepRelativeOffset" false 2.0 1.0 0.0 null null))
  (set `self.MovingSound` _returnvalue)
  (`self.OnSpawn`)
  (switch `/Game/TestTurtles/Blueprints/TurtleBP/ETurtleType` (`self.TurtleType`)
    (:`NewEnumerator0`
      (`self.MoveToFinishSimple`))
    (:`NewEnumerator1`
      (`self.MoveToFinishDelayed`))
    (:`NewEnumerator2`
      (`self.MoveToFinishBackAndForth`))))

(event `MoveToFinishSimple`
  ;[1 1 1] Movement Functions
  (`AIBlueprintHelperLibrary.SimpleMoveToActor` (`self.GetController`) (`self.FinishPoint`)))

(event `MoveToFinishDelayed`
  ;[1 1 1] Movement Functions
  (`AIBlueprintHelperLibrary.SimpleMoveToActor` (`self.GetController`) (`self.FinishPoint`) :!label _label)
  (`KismetSystemLibrary.Delay` 1.0)
  (`Controller.StopMovement` (`self.GetController`))
  (`KismetSystemLibrary.Delay` 0.5)
  (goto _label))

(event `MoveToFinishBackAndForth`
  ;[1 1 1] Movement Functions
  (`AIBlueprintHelperLibrary.SimpleMoveToActor` (`self.GetController`) (`self.FinishPoint`) :!label _label_2)
  (`KismetSystemLibrary.Delay` 1.0)
  (`AIBlueprintHelperLibrary.SimpleMoveToActor` (`self.GetController`) (`self.StartingPoint`))
  (`KismetSystemLibrary.Delay` 0.5)
  (goto _label_2))

(event `OnSpawn`
  ;[1 1 1] Spawn and destroy effects
  (`NiagaraFunctionLibrary.SpawnSystemAtLocation` "/Game/TestTurtles/Niagara/TurtleSpawnSystem.TurtleSpawnSystem" (`self.K2_GetActorLocation`))
  (`GameplayStatics.PlaySoundAtLocation` "/Game/TestTurtles/Sounds/SpawnCue.SpawnCue" (`self.K2_GetActorLocation`) (struct) 1.0 1.0 0.0 null null null))

(event `OnDestroy`
  ;[1 1 1] Spawn and destroy effects
  (`NiagaraFunctionLibrary.SpawnSystemAtLocation` "/Game/TestTurtles/Niagara/TurtleExplotionSystem.TurtleExplotionSystem" (`self.K2_GetActorLocation`))
  (`GameplayStatics.PlaySoundAtLocation` "/Game/StarterContent/Audio/Explosion_Cue.Explosion_Cue" (`self.K2_GetActorLocation`) (struct) 1.0 1.0 0.0 null null null)
  (`AudioComponent.Stop` (`self.MovingSound`))
  (`self.K2_DestroyActor`))

(event `self.ReceiveTick`
  (params (DeltaSeconds :type "Float (single-precision)"))
  ;[1 1 1] Check should the moving sound play
  (`AudioComponent.SetPaused` (`self.MovingSound`) (< (`KismetMathLibrary.VSize` (`self.GetVelocity`)) 5.0)))

(fn `UserConstructionScript`)
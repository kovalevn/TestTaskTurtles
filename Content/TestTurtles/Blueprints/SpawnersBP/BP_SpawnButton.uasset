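; Numbered spawn button that, when activated, plays a press animation and tells its connected nest to spawn a turtle.
; An overlap volume adds and removes the button from the character's InteractableButtons list.
; Activate uses a DoOnce reset after a short delay as a cooldown; without a valid nest it prints an error and never resets.
; A timeline lerps the mesh for the press, and the construction script displays the button number.
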(event `self.ReceiveBeginPlay`
  (bind _output_get (set `self.ButtonStartPoint` (`SceneComponent.K2_GetComponentLocation` (`self.Button`))))
  (set `self.ButtonEndPoint` (`KismetMathLibrary.MakeVector` (.x _output_get) (.y _output_get) (- (.z _output_get) 12.0))))

(event `Activate`
  (`/Engine/EditorBlueprintResources/StandardMacros.DoOnce` false :!label _label
    (:`Completed`
      (`/Engine/EditorBlueprintResources/StandardMacros.IsValid` (`self.ConnectedNest`)
        (:`Is Valid`
          (`self.MoveButton`)
          (`/Game/TestTurtles/Blueprints/SpawnersBP/BP_Nest.SpawnTurtle` (`self.ConnectedNest`))
          (`KismetSystemLibrary.Delay` 1.0)
          (goto _label :!via `Reset`))
        (:`Is Not Valid`
          (`KismetSystemLibrary.PrintString` "No nest assigned to choosen button!" true true (struct :`R` 1.0 :`A` 1.0)))))))

(event `self.InteractCollision.OnComponentBeginOverlap`
  (params (OverlappedComponent :type "PrimitiveComponent Object Reference") (OtherActor :type "Actor Object Reference") (OtherComp :type "PrimitiveComponent Object Reference") (OtherBodyIndex :type Integer) (bFromSweep :type Boolean) (SweepResult :type "HitResult Structure (by ref)"))
  (bind _asthird_person_character (cast `/Game/TestTurtles/Blueprints/CharacterBP/ThirdPersonCharacter` OtherActor))
  (`KismetArrayLibrary.Array_AddUnique` (`/Game/TestTurtles/Blueprints/CharacterBP/ThirdPersonCharacter.InteractableButtons` _asthird_person_character) self))

(event `self.InteractCollision.OnComponentEndOverlap`
  (params (OverlappedComponent :type "PrimitiveComponent Object Reference") (OtherActor :type "Actor Object Reference") (OtherComp :type "PrimitiveComponent Object Reference") (OtherBodyIndex :type Integer))
  (bind _asthird_person_character (cast `/Game/TestTurtles/Blueprints/CharacterBP/ThirdPersonCharacter` OtherActor))
  (`KismetArrayLibrary.Array_RemoveItem` (`/Game/TestTurtles/Blueprints/CharacterBP/ThirdPersonCharacter.InteractableButtons` _asthird_person_character) self))

(event `MoveButton`
  ;[1 1 1] Button press animation
  (bind (_direction _location) (`Timeline|MoveButtonTimeline` :!via `PlayFromStart`)
    (:`Update`
      (`SceneComponent.K2_SetWorldLocation` (`self.Button`) (`KismetMathLibrary.VLerp` (`self.ButtonEndPoint`) (`self.ButtonStartPoint`) _location) false false))))

(fn `UserConstructionScript`
  (`TextRenderComponent.K2_SetText` (`self.TextRender`) (`self.ButtonNumber`)))
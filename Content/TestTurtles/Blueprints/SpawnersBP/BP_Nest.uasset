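; BP_Nest is a turtle spawner that launches turtles toward an assigned finish point.
; Its SpawnTurtle event spawns a BP_Turtle slightly above the nest, passing in the movement type, the nest as starting point and the finish point.
; If no valid finish point is assigned, it prints an error instead.
; The construction script shows the nest's button number on a text render component.
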(event `SpawnTurtle`
  (bind (_returnvalue_x _returnvalue_y _returnvalue_z) (`KismetMathLibrary.BreakVector` (`self.K2_GetActorLocation`)))
  (`/Engine/EditorBlueprintResources/StandardMacros.IsValid` (`self.Finish`)
    (:`Is Valid`
      (`|SpawnActorFromClass` "/Game/TestTurtles/Blueprints/TurtleBP/BP_Turtle.BP_Turtle_C" (`KismetMathLibrary.MakeTransform` (`KismetMathLibrary.MakeVector` _returnvalue_x _returnvalue_y (+ _returnvalue_z 50.0))) "Undefined" "OverrideRootScale" null (`self.TurtleMovementType`) self (`self.Finish`) null))
    (:`Is Not Valid`
      (`KismetSystemLibrary.PrintString` "No finish point assigned to choosen button's nest!" true true (struct :`R` 1.0 :`A` 1.0)))))

(fn `UserConstructionScript`
  (`TextRenderComponent.K2_SetText` (`self.TextRender`) (`self.ButtonNumber`)))